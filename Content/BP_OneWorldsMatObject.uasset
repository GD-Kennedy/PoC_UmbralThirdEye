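; BP_OneWorldsMatObject is a static mesh object whose collision depends on whether the player's alternate world is active.
; One tick after BeginPlay it binds to the third-person character's AltWorldToggled event and sets its initial collision response.
; Each toggle switches GameTraceChannel1 between Block and Ignore, with an Inverted flag choosing in which world the object blocks.
; Only collision changes here; no material or visibility logic is present.
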(event `self.ReceiveBeginPlay`
  ;[1 1 1] Bind to player toggle event
  (`KismetSystemLibrary.DelayUntilNextTick`) ; To ensure that player is already spawned.
  (bind _asbp_third_person_character (cast `/Game/ThirdPerson/Blueprints/BP_ThirdPersonCharacter` (`GameplayStatics.GetPlayerCharacter` 0)))
  (add `/Game/ThirdPerson/Blueprints/BP_ThirdPersonCharacter.AltWorldToggled` _asbp_third_person_character (delegate `OnToggled`))
  (`PrimitiveComponent.SetCollisionResponseToChannel` (`self.StaticMesh`) "ECC_GameTraceChannel1" (select `bool` (`self.Inverted`) :`false` "ECR_Block" :`true` "ECR_Ignore" :!type "ECollisionResponse Enum")))

(event `OnToggled`
  (params (Enabled :type Boolean))
  ;[1 1 1] Adjust collision in response
  (`PrimitiveComponent.SetCollisionResponseToChannel` (`self.StaticMesh`) "ECC_GameTraceChannel1" (select `bool` (xor Enabled (`self.Inverted`)) :`false` "ECR_Block" :`true` "ECR_Ignore" :!type "ECollisionResponse Enum")))

(fn `UserConstructionScript`)